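; VR player controller that detects an HMD, then spawns and possesses a simple VR character.
; InitiatePlay checks for a connected headset in VR preview or game, reports it through ReturnHMDStatus, and prints the player ID.
; If an HMD is present, the pawn spawns with team 0 at a random TeamPlayerStart matching the controller's TeamID.
; InitHMD is then called with false, so it skips enabling the HMD.
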(event `InitiatePlay`
  (`self.GetHMDStatus`)
  (`KismetSystemLibrary.PrintString` (`KismetStringLibrary.Concat_StrStr` "Your ID is " (`KismetStringLibrary.Conv_IntToString` (`PlayerState.PlayerId` (`self.PlayerState`))))))

(event `GetHMDStatus`
  (`self.ReturnHMDStatus` (and (`VRExpansionFunctionLibrary.GetIsHMDConnected`) (`VRExpansionFunctionLibrary.IsInVREditorPreviewOrGame`))))

(event `ReturnHMDStatus`
  (params (HMDEnabled :type Boolean))
  (bind _output_get (set `self.HMDEnabled` HMDEnabled))
  (if _output_get
    ;[1 1 1] Spawn Player Character and possess
    (bind _item (`self.ChooseSpawnLoc`))
    (bind _returnvalue (`|SpawnActorFromClass` "/Game/Blueprints/VRPlayerCharacterSimple.VRPlayerCharacterSimple_C" (`self.GetTransform` _item) "Undefined" "OverrideRootScale" self))
    (`self.Possess` _returnvalue)
    (`self.InitHMD` false)))

(event `InitHMD`
  (params (HasHMD :type Boolean))
  (if HasHMD
    (`HeadMountedDisplayFunctionLibrary.EnableHMD` true)))

(fn `ChooseSpawnLoc`
  (returns (Item :type "/Game/Blueprints/GameplayBP/TeamPlayerStart Object Reference"))
  (bind _outactors (`GameplayStatics.GetAllActorsOfClass` "/Game/Blueprints/GameplayBP/TeamPlayerStart.TeamPlayerStart_C"))
  (bind (_arrayindex _arrayelement) (`/Engine/EditorBlueprintResources/StandardMacros.ReverseForEachLoop` _outactors)
    (:`LoopBody`
      (bind _teamid (message `/Game/Blueprints/TeamInterface.GetTeamID` _arrayelement))
      (if (!= _teamid (`self.TeamID`))
        (`KismetArrayLibrary.Array_RemoveItem` _outactors _arrayelement)))
    (:`Completed`
      (return (`KismetArrayLibrary.Array_Get` _outactors (`KismetMathLibrary.RandomIntegerInRange` 0 (- (`KismetArrayLibrary.Array_Length` _outactors) 1)))))))

(fn `UserConstructionScript`)