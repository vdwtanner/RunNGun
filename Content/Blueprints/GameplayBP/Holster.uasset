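; VR weapon holster actor that stores one gun and detects the player's motion-controller hands.
; Box overlap by a hand with grip unpressed pulses that controller and registers the holster on the player character; SetHolsterActive toggles the box's collision.
; PlaceGunInHolster drops any held gun and snap-attaches the new one, while SwapGuns also returns the previous gun.
; DropGun detaches the gun, then enables physics or optionally destroys it if empty.
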(event `self.Box.OnComponentBeginOverlap`
  (params (OverlappedComponent :type "PrimitiveComponent Object Reference") (OtherActor :type "Actor Object Reference") (OtherComp :type "PrimitiveComponent Object Reference") (OtherBodyIndex :type Integer) (bFromSweep :type Boolean) (SweepResult :type "HitResult Structure (by ref)"))
  (bind _asgrip_motion_controller_component (cast `GripMotionControllerComponent` (`KismetArrayLibrary.Array_Get` (`SceneComponent.GetParentComponents` OtherComp))))
  (bind _asvrplayer_character_simple (cast `/Game/Blueprints/VRPlayerCharacterSimple` OtherActor))
  (switch `EControllerHand` (`GripMotionControllerComponent.Hand` _asgrip_motion_controller_component)
    (:`Left`
      (if (not (`/Game/Blueprints/VRPlayerCharacterSimple.LeftGripPressed` _asvrplayer_character_simple))
        (bind _returnvalue (`GameplayStatics.GetPlayerController` _asvrplayer_character_simple))
        (`PlayerController.ClientPlayForceFeedback` _returnvalue "/Game/Blueprints/LeftControllerHapticPulse.LeftControllerHapticPulse" false "None")
        (set `/Game/Blueprints/VRPlayerCharacterSimple.LeftHandInHolster` self _asvrplayer_character_simple)))
    (:`Right`
      (if (not (`/Game/Blueprints/VRPlayerCharacterSimple.RightGripPressed` _asvrplayer_character_simple))
        (`PlayerController.ClientPlayForceFeedback` _returnvalue "/Game/Blueprints/RightControllerHapticPulse.RightControllerHapticPulse" false "None")
        (set `/Game/Blueprints/VRPlayerCharacterSimple.RightHandInHolster` self _asvrplayer_character_simple)))))

(event `SetHolsterActive`
  (params (Active :type Boolean))
  (bind _box (`self.Box`))
  (if Active
    (`PrimitiveComponent.SetCollisionEnabled` _box "QueryOnly")
    (else
      (`PrimitiveComponent.SetCollisionEnabled` _box "NoCollision"))))

(fn `DropGun`
  (params (DestroyIfEmpty :type Boolean :default true))
  (bind _gunbaseref (`self.GunBaseRef`))
  (bind _gun (`/Game/Blueprints/GameplayBP/Weapons/GunBase.Gun` _gunbaseref))
  (if (!= (`self.GunBaseRef`) null)
    (`self.K2_DetachFromActor` _gunbaseref "KeepWorld" "KeepWorld" "KeepWorld")
    (if (and DestroyIfEmpty (not (`/Game/Blueprints/GameplayBP/Weapons/GunBase.HasAmmo` _gunbaseref)))
      (`self.K2_DestroyActor` _gunbaseref)
      (else
        (`PrimitiveComponent.SetCollisionEnabled` _gun "QueryAndPhysics")
        (`PrimitiveComponent.SetSimulatePhysics` _gun true)
        (set `self.GunBaseRef` null)))))

(fn `PlaceGunInHolster`
  (params (GunToPlace :type "/Game/Blueprints/GameplayBP/Weapons/GunBase Object Reference"))
  (if (!= (`self.GunBaseRef`) null)
    (`self.DropGun` false))
  (bind _output_get (set `self.GunBaseRef` GunToPlace))
  (`PrimitiveComponent.SetCollisionEnabled` (`/Game/Blueprints/GameplayBP/Weapons/GunBase.Gun` _output_get) "QueryOnly")
  (`self.K2_AttachToActor` (`self.GunBaseRef`) self "None" "SnapToTarget" "SnapToTarget" "KeepWorld" true))

(fn `SwapGuns`
  (params (WeaponToPutInHolster :type "/Game/Blueprints/GameplayBP/Weapons/GunBase Object Reference"))
  (returns (WeaponRetrievedFromHolster :type "/Game/Blueprints/GameplayBP/Weapons/GunBase Object Reference"))
  (locals (GunBaseTemp :type "/Game/Blueprints/GameplayBP/Weapons/GunBase Object Reference"))
  (bind _output_get (set `local.GunBaseTemp` (`self.GunBaseRef`)))
  (`self.PlaceGunInHolster` WeaponToPutInHolster) ; Automatically drops old gun
  (return _output_get))

(fn `UserConstructionScript`)